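; Tower defense enemy actor that follows a spline path and dies when its health runs out.
; Each tick it advances distance along the spline supplied through SetSpline by MovementSpeed, taking X, Y and rotation from the spline but keeping its own height and scale.
; AnyDamage lowers clamped health unless IsDead is set, and at zero Die calls the OnEnemyDied dispatcher with itself before destroying the actor.
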(event `self.ReceiveBeginPlay`
  (set `self.CurrentHealth` (`self.MaxHealth`)))

(event `self.ReceiveTick`
  (params (DeltaSeconds :type "Float (single-precision)"))
  (`/Engine/EditorBlueprintResources/StandardMacros.IsValid` (`self.SplineRef`)
    (:`Is Valid`
      (`self.MoveEnemyOnSpline` DeltaSeconds))))

(event `self.ReceiveAnyDamage`
  (params (Damage :type "Float (single-precision)") (DamageType :type "DamageType Object Reference") (InstigatedBy :type "Controller Object Reference") (DamageCauser :type "Actor Object Reference"))
  (if (not (`self.IsDead`))
    (bind _output_get (set `self.CurrentHealth` (`KismetMathLibrary.FClamp` (- (`self.CurrentHealth`) Damage) 0.0 (`self.MaxHealth`))))
    (if (<= _output_get 0.0)
      (`self.Die`))))

(fn `Die`
  (`self.OnEnemyDied` self)
  (`self.K2_DestroyActor`))

(fn `MoveEnemyOnSpline`
  (params (DeltaSeconds :type "Float (double-precision)"))
  (bind (_returnvalue_location _returnvalue_rotation) (`KismetMathLibrary.BreakTransform` (`SplineComponent.GetTransformAtDistanceAlongSpline` (`self.SplineRef`) (`self.Distance Along Spline`) "World" false)))
  (set `self.Distance Along Spline` (+ (* DeltaSeconds (`self.MovementSpeed`)) (`self.Distance Along Spline`)))
  (`SceneComponent.K2_SetRelativeTransform` (`self.RootComponent`) (`KismetMathLibrary.MakeTransform` (`KismetMathLibrary.MakeVector` (.x _returnvalue_location) (.y _returnvalue_location) (.z (`self.K2_GetActorLocation`))) _returnvalue_rotation (`self.GetActorScale3D`)) false false))

(fn `SetSpline`
  (params (Spline :type "SplineComponent Object Reference"))
  (set `self.SplineRef` Spline))

(fn `UserConstructionScript`)