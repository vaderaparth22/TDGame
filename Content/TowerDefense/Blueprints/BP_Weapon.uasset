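; Tower defense weapon that automatically damages one BP_Enemy at a time within its attack range sphere.
; Sphere overlaps maintain the in-range list and bind to each enemy's death event, which removes it and clears the current target.
; A looping timer started at BeginPlay calls Attack, which applies damage directly to a valid target or otherwise searches for a new one by highest PathProgress.
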(event `self.ReceiveBeginPlay`
  (`KismetSystemLibrary.K2_SetTimer` null "Attack" 0.5 true))

(event `self.AttackRangeSphere.OnComponentBeginOverlap`
  (params (OverlappedComponent :type "PrimitiveComponent Object Reference") (OtherActor :type "Actor Object Reference") (OtherComp :type "PrimitiveComponent Object Reference") (OtherBodyIndex :type Integer) (bFromSweep :type Boolean) (SweepResult :type "HitResult Structure (by ref)"))
  (bind _asbp_enemy (cast `/Game/TowerDefense/Blueprints/BP_Enemy` OtherActor))
  (`/Engine/EditorBlueprintResources/StandardMacros.IsValid` _asbp_enemy
    (:`Is Valid`
      (`KismetArrayLibrary.Array_AddUnique` (`self.EnemiesInRange`) _asbp_enemy)
      (add `/Game/TowerDefense/Blueprints/BP_Enemy.OnEnemyDied` _asbp_enemy (delegate `HandleEnemyDied`)))))

(event `HandleEnemyDied`
  (params (EnemyReference :type "/Game/TowerDefense/Blueprints/BP_Enemy Object Reference"))
  (`KismetArrayLibrary.Array_RemoveItem` (`self.EnemiesInRange`))
  (if (== EnemyReference (`self.CurrentTarget`))
    (set `self.CurrentTarget` null)
    (`KismetSystemLibrary.PrintString` "Enemy killed")))

(event `self.AttackRangeSphere.OnComponentEndOverlap`
  (params (OverlappedComponent :type "PrimitiveComponent Object Reference") (OtherActor :type "Actor Object Reference") (OtherComp :type "PrimitiveComponent Object Reference") (OtherBodyIndex :type Integer))
  (bind _asbp_enemy (cast `/Game/TowerDefense/Blueprints/BP_Enemy` OtherActor))
  (`/Engine/EditorBlueprintResources/StandardMacros.IsValid` _asbp_enemy
    (:`Is Valid`
      (`KismetArrayLibrary.Array_RemoveItem` (`self.EnemiesInRange`) _asbp_enemy)
      (if (== (`self.CurrentTarget`) _asbp_enemy)
        (set `self.CurrentTarget` null)
        (clear `/Game/TowerDefense/Blueprints/BP_Enemy.OnEnemyDied` _asbp_enemy)))))

(fn `Attack`
  (bind _currenttarget (`self.CurrentTarget`))
  (`/Engine/EditorBlueprintResources/StandardMacros.IsValid` _currenttarget
    (:`Is Valid`
      (`GameplayStatics.ApplyDamage` _currenttarget (`self.BaseDamage`) null self))
    (:`Is Not Valid`
      (`self.FindNewTarget`))))

(fn `FindNewTarget`
  (locals (BestEnemy :type "TDEnemy Object Reference") (HighestProgress :type "Float (double-precision)" :default -1.0))
  (bind _enemiesinrange (`self.EnemiesInRange`))
  (if (`KismetArrayLibrary.Array_IsNotEmpty` _enemiesinrange)
    (for _array_element _enemiesinrange
      (`/Engine/EditorBlueprintResources/StandardMacros.IsValid` _array_element
        (:`Is Valid`
          (bind _asbp_enemy (cast `/Game/TowerDefense/Blueprints/BP_Enemy` _array_element))
          (if (> (`/Game/TowerDefense/Blueprints/BP_Enemy.PathProgress` _asbp_enemy) (`local.HighestProgress`))
            (set `local.HighestProgress` (`/Game/TowerDefense/Blueprints/BP_Enemy.PathProgress` _asbp_enemy))
            (bind _output_get (set `local.BestEnemy` _asbp_enemy))
            (set `self.CurrentTarget` _output_get)))))))

(fn `UserConstructionScript`)